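; Actor component that switches the player's camera between third-person, shoulder, first-person, top-down, isometric and CCTV views.
; UpdateCameraState gates changes and loads DT_CameraInfo rows, while CameraTransition lerps spring arm, FOV and rotation from an externally supplied alpha.
; FinishTransition commits the state, swapping the skeletal mesh for first person or the active camera for true first person.
; CCTV bypasses transitions, toggling look input and ticking to keep the nearest BP_CCTV_Camera in use.
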(event EventTick
  (params (DeltaSeconds :type Float%20%28single-precision%29))
  ;[1 1 1] Event tick only active whilst CCTV active and then this is checking what the closest CCTV camera is and setting that to be the one in use and the others to not be in use anymore
  (bind _outactors (Actor|GetAllActorsOfClass "/Game/Camera_System/BP_CCTV_Camera.BP_CCTV_Camera_C"))
  (Class|BPICCTVCameras|UpdateinUse(Message) (.ReturnValue (Actor|FindNearestActor (Transformation|GetActorLocation (Components|GetOwner)) _outactors)) true (.ReturnValue (Actor|FindNearestActor (Transformation|GetActorLocation (Components|GetOwner)) _outactors)))
  (for _array_element _outactors
    (if (!= _array_element (.ReturnValue (Actor|FindNearestActor (Transformation|GetActorLocation (Components|GetOwner)) _outactors)))
      (Class|BPICCTVCameras|UpdateinUse(Message) _array_element false (.ReturnValue (Actor|FindNearestActor (Transformation|GetActorLocation (Components|GetOwner)) _outactors))))))

(fn UpdateCameraState
  (params (New_Camera_State :type Enum_Camera_States%20Enum :default "NewEnumerator0"))
  ;[1 1 1] Can only start a state change if not already transitioning
  (if (Variables|CurrentProcess|GetTransitioning)
    ;[1 1 1] Return false so transition doesn't start
    (return false)
    (else
      ;[1 1 1] Set new camera state and reset alpha
      (bind _output_get (Variables|States|SetNew_Camera_State New_Camera_State))
      (Variables|Lerping|SetAlpha 0.0)
      ;[1 1 1] IF CCTV
      (if (Utilities|Enum|Equal(Enum) _output_get "NewEnumerator7")
        ;[1 1 1] If CCTV is already active
        (if (Variables|CCTV|GetCCTVActive)
          ;[1 1 1] Deactivate CCTV
          (CallFunction|DeactivateCCTV)
          ;[1 1 1] Disable tick
          (Components|Tick|SetComponentTickEnabled false)
          ;[1 1 1] Update CCTV active
          (Variables|CCTV|SetCCTVActive false)
          ;[1 1 1] Change the camera state to third person
          (Class|BPICameraSystem|ChangeCameraState(Message) (Game|GetPlayerCharacter 0) "NewEnumerator0")
          (else
            ;[1 1 1] Check if any CCTV cameras in level
            (bind _outactors (Actor|GetAllActorsOfClass "/Game/Camera_System/BP_CCTV_Camera.BP_CCTV_Camera_C"))
            (if (Utilities|Array|IsEmpty _outactors)
              ;[1 1 1] Deactivate CCTV
              (CallFunction|DeactivateCCTV)
              ;[1 1 1] Disable tick
              (Components|Tick|SetComponentTickEnabled false)
              ;[1 1 1] Update CCTV active
              (Variables|CCTV|SetCCTVActive false)
              (else
                ;[1 1 1] Update CCTV active
                (Variables|CCTV|SetCCTVActive true)
                ;[1 1 1] Set tick enabled
                (Components|Tick|SetComponentTickEnabled true)
                ;[1 1 1] Update nearest CCTV camera to be the one in use
                (Class|BPICCTVCameras|UpdateinUse(Message) (.ReturnValue (Actor|FindNearestActor (Transformation|GetActorLocation (Components|GetOwner)) _outactors)) true)
                ;[1 1 1] Ignore look input whilst in CCTV
                (Input|SetIgnoreLookInput (Game|GetPlayerController 0) true)
                ;[1 1 1] Return false since the transition is using the cctv camera blueprint instead of stats from the data table
                (return false)))))
        ;[1 1 1] Reset ignore look input
        (Input|SetIgnoreLookInput (Game|GetPlayerController 0) false)
        ;[1 1 1] Return false so transition doesn't start for CCTV
        (return false)
        (else
          ;[1 1 1] Reset ignore look input
          (Input|SetIgnoreLookInput (Game|GetPlayerController 0) false)
          ;[1 1 1] Start the camera state transition
          (CallFunction|StartTransition)
          ;[1 1 1] Deactivate CCTV
          (CallFunction|DeactivateCCTV)
          ;[1 1 1] Set tick enabled
          (Components|Tick|SetComponentTickEnabled false)
          ;[1 1 1] Return true so transition will start
          (return true))))))

(fn CameraTransition
  (params (Alpha :type Float%20%28double-precision%29) (Finished :type Boolean))
  (bind _camera (Variables|Default|GetCamera))
  (bind _new_camera_state (Variables|States|GetNew_Camera_State))
  ;[1 1 1] Update alpha based on passed float
  (Variables|Lerping|SetAlpha Alpha)
  (if Finished
    ;[1 1 1] Finished the transition
    (CallFunction|FinishTransition)
    (else
      (Utilities|FlowControl|Sequence
        (:then_0
          ;[1 1 1] Lerping specified values from old state values to new state values
          ;;[1 1 1] Whilst transitioning
          (Variables|CurrentProcess|SetTransitioning true))
        (:then_1
          (Transformation|SetRelativeLocation (Variables|Default|GetCameraSpringArm) (Math|Vector|Lerp(Vector) (Variables|OldInfo|GetOldSpringArmLocation) (Variables|NewInfo|GetNewSpringArmLocation) (Variables|Lerping|GetAlpha)) false false)
          (Variables|/Script/Engine.SpringArmComponent|SetTargetArmLength (Variables|Default|GetCameraSpringArm) (Math|Float|Lerp (Variables|OldInfo|GetOldTargetArmLength) (Variables|NewInfo|GetNewTargetArmLength) (Variables|Lerping|GetAlpha)))
          (Variables|/Script/Engine.SpringArmComponent|SetSocketOffset (Variables|Default|GetCameraSpringArm) (Math|Vector|Lerp(Vector) (Variables|OldInfo|GetOldSocketOffset) (Variables|NewInfo|GetNewSocketOffset) (Variables|Lerping|GetAlpha)))
          (Variables|/Script/Engine.SpringArmComponent|SetTargetOffset (Variables|Default|GetCameraSpringArm) (Math|Vector|Lerp(Vector) (Variables|OldInfo|GetOldTargetOffset) (Variables|NewInfo|GetNewTargetOffset) (Variables|Lerping|GetAlpha)))
          (Variables|/Script/Engine.CameraComponent|SetFieldOfView (Variables|Default|GetCamera) (Math|Float|Lerp (Variables|OldInfo|GetOldFieldOfView) (Variables|NewInfo|GetNewFieldOfView) (Variables|Lerping|GetAlpha)))
          (if (or (Utilities|Enum|Equal(Enum) _new_camera_state "NewEnumerator5") (Utilities|Enum|Equal(Enum) _new_camera_state "NewEnumerator6"))
            (Transformation|SetRelativeRotation _camera (Math|Rotator|Lerp(Rotator) (Variables|/Script/Engine.SceneComponent|GetRelativeRotation (Variables|Default|GetCamera)) (Math|Rotator|SelectRotator (Math|Rotator|MakeRotator 0.0 (.pitch (Math|Rotator|FindLookatRotation (Transformation|GetWorldLocation (Variables|Default|GetCamera)) (Transformation|GetActorLocation (Components|GetOwner)))) 0.0) "-35.000000,0.000000,0.000000" (Utilities|Enum|Equal(Enum) (Variables|States|GetNew_Camera_State) "NewEnumerator5")) (Variables|Lerping|GetAlpha)) false false)
            (else
              (Transformation|SetRelativeRotation _camera (Math|Rotator|Lerp(Rotator) (Variables|/Script/Engine.SceneComponent|GetRelativeRotation (Variables|Default|GetCamera)) "0, 0, 0" (Variables|Lerping|GetAlpha) true) false false))))))))

(fn StartTransition
  (bind _returnvalue (Game|GetPlayerController 0))
  (bind _cameraspringarm (Variables|Default|GetCameraSpringArm))
  (bind _cameraspringarm_2 (Variables|Default|GetCameraSpringArm))
  ;[1 1 1] Getting info for current state and next state that is being transitioned into
  (bind _returnvalue_2 (Utilities|GetDataTableRow "/Game/Camera_System/DT_CameraInfo.DT_CameraInfo" (Utilities|String|StringToName (Utilities|String|EnumtoString (Variables|States|GetCurrent_Camera_State))))
    (:then
      (Utilities|UpdateOldInfo (.springarmlocation _returnvalue_2) (.targetarmlength _returnvalue_2) (.socketoffset _returnvalue_2) (.targetoffset _returnvalue_2) (.fieldofview _returnvalue_2)
        (:Done
          (bind _returnvalue_3 (Utilities|GetDataTableRow "/Game/Camera_System/DT_CameraInfo.DT_CameraInfo" (Utilities|String|StringToName (Utilities|String|EnumtoString (Variables|States|GetNew_Camera_State))))
            (:then
              (Utilities|UpdateNewInfo (.springarmlocation _returnvalue_3) (.targetarmlength _returnvalue_3) (.socketoffset _returnvalue_3) (.targetoffset _returnvalue_3) (.fieldofview _returnvalue_3)
                (:Done
                  ;[1 1 1] Update camera to be the true first person camera if the state to be transitioned to is the truefirstperson state
                  (if (Utilities|Enum|Equal(Enum) (Variables|States|GetNew_Camera_State) "NewEnumerator3")
                    _
                    (else
                      (Components|Activation|SetActive (Variables|Default|GetTrueFirstPersonCamera) false false)
                      (Components|Activation|SetActive (Variables|Default|GetCamera) true false)))
                  ;[1 1 1] Update all one time necessary stats for the new state
                  (bind _returnvalue_4 (Utilities|GetDataTableRow "/Game/Camera_System/DT_CameraInfo.DT_CameraInfo" (Utilities|String|StringToName (Utilities|String|EnumtoString (Variables|States|GetNew_Camera_State))))
                    (:then
                      (Variables|/Script/Engine.SpringArmComponent|SetbEnableCameraLag (Variables|Default|GetCameraSpringArm) (.cameralag _returnvalue_4))
                      (Variables|/Script/Engine.SpringArmComponent|SetCameraLagSpeed (Variables|Default|GetCameraSpringArm) (.cameralagspeed _returnvalue_4))
                      (Variables|/Script/Engine.SpringArmComponent|SetbEnableCameraRotationLag (Variables|Default|GetCameraSpringArm) (.camerarotationlag _returnvalue_4))
                      (Variables|/Script/Engine.SpringArmComponent|SetCameraRotationLagSpeed (Variables|Default|GetCameraSpringArm) (.camerarotationlagspeed _returnvalue_4))
                      (Class|CameraComponent|SetProjectionMode (Variables|Default|GetCamera) (select (.projectionmodeperspective _returnvalue_4) "Perspective" "Orthographic"))
                      (bind _aspawn (Utilities|Casting|CastToPawn (Components|GetOwner)))
                      (Variables|/Script/Engine.Pawn|SetbUseControllerRotationYaw _aspawn (.usecontrollerrotationyaw _returnvalue_4))
                      ;[1 1 1] Switch on camera states for new camera state
                      (switch Utilities|FlowControl|Switch|SwitchonEnum_Camera_States (Variables|States|GetNew_Camera_State)
                        (:NewEnumerator0
                          ;[1 1 1] Ignore look input if transitioning into topdown, isometric or CCTV state
                          (Input|SetIgnoreLookInput _returnvalue false :!label _label)
                          ;[1 1 1] Update camera spring arm states dependant on state being transitioned into
                          (Variables|/Script/Engine.SpringArmComponent|SetbUsePawnControlRotation _cameraspringarm_2 true)
                          (Variables|/Script/Engine.SpringArmComponent|SetbInheritPitch _cameraspringarm true)
                          (Variables|/Script/Engine.SpringArmComponent|SetbInheritRoll _cameraspringarm true)
                          (Variables|/Script/Engine.SpringArmComponent|SetbInheritYaw _cameraspringarm true))
                        (:NewEnumerator1
                          (goto _label))
                        (:NewEnumerator8
                          (goto _label))
                        (:NewEnumerator2
                          (goto _label))
                        (:NewEnumerator3
                          (goto _label))
                        (:NewEnumerator4
                          (goto _label))
                        (:NewEnumerator5
                          (Utilities|FlowControl|Sequence :!label _label_2
                            (:then_0
                              (Input|SetIgnoreLookInput _returnvalue true :!label _label_3))
                            (:then_1
                              (Variables|/Script/Engine.SpringArmComponent|SetbUsePawnControlRotation _cameraspringarm_2 false)
                              (Variables|/Script/Engine.SpringArmComponent|SetbInheritPitch _cameraspringarm false)
                              (Variables|/Script/Engine.SpringArmComponent|SetbInheritRoll _cameraspringarm false)
                              (Variables|/Script/Engine.SpringArmComponent|SetbInheritYaw _cameraspringarm false))))
                        (:NewEnumerator6
                          (goto _label_2))
                        (:NewEnumerator7
                          (goto _label_3))))
                    (:RowNotFound
                      (Development|PrintString "ROW NOT FOUND FOR STARTING TRANSITION"))))))
            (:RowNotFound
              (Development|PrintString "row not found for state to transition to"))))))
    (:RowNotFound
      (Development|PrintString "row not found for current state"))))

(fn SetupCameraSystem
  (params (Camera :type Camera%20Component%20Object%20Reference) (Mesh :type Skeletal%20Mesh%20Component%20Object%20Reference) (Camera%20Spring%20Arm :type Spring%20Arm%20Component%20Object%20Reference) (Capsule%20Component :type Capsule%20Component%20Object%20Reference) (FirstPersonModel :type Skeletal%20Mesh%20Object%20Reference) (ThirdPersonModel :type Skeletal%20Mesh%20Object%20Reference) (TrueFirstPersonCamera :type Camera%20Component%20Object%20Reference))
  ;[1 1 1] Setup required components and models for this to work
  (Variables|Default|SetCamera Camera)
  (Variables|Default|SetMesh Mesh)
  (Variables|Default|SetCameraSpringArm Camera%20Spring%20Arm)
  (Variables|Default|SetCapsuleComponent Capsule%20Component)
  (Variables|Models|SetFirstPersonModel FirstPersonModel)
  (Variables|Models|SetThirdPersonModel ThirdPersonModel)
  (Variables|Default|SetTrueFirstPersonCamera TrueFirstPersonCamera))

(fn FinishTransition
  (bind _mesh (Variables|Default|GetMesh))
  ;[1 1 1] Finish transition and set the current state to be the new state that was transitioned into and then set the transitioning bool to be false so can transition into another state
  (bind _output_get (Variables|States|SetCurrent_Camera_State (Variables|States|GetNew_Camera_State)))
  (Variables|CurrentProcess|SetTransitioning false)
  ;[1 1 1] Update character skeletal mesh model depending on if in the first person state
  (if (Utilities|Enum|Equal(Enum) _output_get "NewEnumerator2")
    (Components|SkeletalMesh|SetSkeletalMeshAsset _mesh (Variables|Models|GetFirstPersonModel))
    (else
      (Components|SkeletalMesh|SetSkeletalMeshAsset _mesh (Variables|Models|GetThirdPersonModel))
      ;[1 1 1] if in true first person state then change the active camera to be the true first person camera and set the base camera to be inactive
      (if (Utilities|Enum|Equal(Enum) _output_get "NewEnumerator3")
        (Components|Activation|SetActive (Variables|Default|GetTrueFirstPersonCamera) true false)
        (Components|Activation|SetActive (Variables|Default|GetCamera) false false)))))

(fn DeactivateCCTV
  ;[1 1 1] Set all CCTV cameras to not be in use since CCTV is deactivated
  (bind _outactors (Actor|GetAllActorsOfClass "/Game/Camera_System/BP_CCTV_Camera.BP_CCTV_Camera_C"))
  (for _array_element _outactors
    (Default|UpdateinUse _array_element false))
  (Development|PrintString "CCTV DEACTIVATED"))