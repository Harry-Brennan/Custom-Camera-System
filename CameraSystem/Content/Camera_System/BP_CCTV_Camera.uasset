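; CCTV camera actor that takes over the player's view with a timed blend and rotates to follow the player character.
; UpdateInUse toggles Tick and routes to Activate or Deactivate, which use paired DoOnce gates and blend out to a supplied camera or back to the player.
; Tick points the spring arm at the player, pausing while the player overlaps the left or right extent volumes.
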(event OnComponentBeginOverlap(StopTrackingExtentLeft)
  (params (OverlappedComponent :type Primitive%20Component%20Object%20Reference) (OtherActor :type Actor%20Object%20Reference) (OtherComp :type Primitive%20Component%20Object%20Reference) (OtherBodyIndex :type Integer) (bFromSweep :type Boolean) (SweepResult :type Hit%20Result%20Structure%20%28by%20ref%29))
  ;[1 1 1] Collision overlaps for tracking extents
  (if (== OtherActor (Game|GetPlayerCharacter 0))
    (Variables|Default|SetshouldTrack false)))

(event OnComponentBeginOverlap(StopTrackingExtentRight)
  (params (OverlappedComponent :type Primitive%20Component%20Object%20Reference) (OtherActor :type Actor%20Object%20Reference) (OtherComp :type Primitive%20Component%20Object%20Reference) (OtherBodyIndex :type Integer) (bFromSweep :type Boolean) (SweepResult :type Hit%20Result%20Structure%20%28by%20ref%29))
  ;[1 1 1] Collision overlaps for tracking extents
  (if (== OtherActor (Game|GetPlayerCharacter 0))
    (Variables|Default|SetshouldTrack false)))

(event OnComponentEndOverlap(StopTrackingExtentRight)
  (params (OverlappedComponent :type Primitive%20Component%20Object%20Reference) (OtherActor :type Actor%20Object%20Reference) (OtherComp :type Primitive%20Component%20Object%20Reference) (OtherBodyIndex :type Integer))
  ;[1 1 1] Collision overlaps for tracking extents
  (if (== OtherActor (Game|GetPlayerCharacter 0))
    (Variables|Default|SetshouldTrack true)))

(event OnComponentEndOverlap(StopTrackingExtentLeft)
  (params (OverlappedComponent :type Primitive%20Component%20Object%20Reference) (OtherActor :type Actor%20Object%20Reference) (OtherComp :type Primitive%20Component%20Object%20Reference) (OtherBodyIndex :type Integer))
  ;[1 1 1] Collision overlaps for tracking extents
  (if (== OtherActor (Game|GetPlayerCharacter 0))
    (Variables|Default|SetshouldTrack true)))

(event EventUpdateinUse
  (params (InUse? :type Boolean) (NewCamera :type Actor%20Object%20Reference))
  ;[1 1 1] Updating this CCTV camera to be in use or no longer in use
  (bind _output_get (Variables|Default|SetinUse InUse?))
  (Actor|Tick|SetActorTickEnabled _output_get)
  (if _output_get
    (CallFunction|Activate)
    (else
      (CallFunction|Deactivate NewCamera))))

(event EventTick
  (params (DeltaSeconds :type Float%20%28single-precision%29))
  ;[1 1 1] Event tick for caling track with event tick only active if the CCTV camera is active
  (if (Variables|Default|GetshouldTrack)
    (CallFunction|Track)))

(event EventTrack
  (bind _returnvalue (Game|GetPlayerCharacter 0))
  (bind _springarm (Variables|Default|GetSpringArm))
  (bind _returnvalue_2 (Transformation|GetActorLocation _returnvalue))
  (bind _returnvalue_3 (Transformation|GetWorldLocation _springarm))
  (bind _returnvalue_4 (Math|Rotator|FindLookatRotation _returnvalue_3 _returnvalue_2))
  ;[1 1 1] Tracking the player
  (Transformation|SetWorldRotation (Variables|Default|GetSpringArm) (Math|Rotator|MakeRotator (.roll _returnvalue_4) (.pitch _returnvalue_4) (.yaw _returnvalue_4)) false false))

(event EventActivate
  ;[1 1 1] Activating and deactivating the camera for setting the view target with blend and updating the isActive bool
  (Utilities|FlowControl|Sequence
    (:then_0
      (Utilities|FlowControl|DoOnce false
        (:Completed
          (Variables|Default|SetisActive true)
          (Game|Player|SetViewTargetwithBlend (Game|GetPlayerController 0) self 1.0 "VTBlend_Linear" 0.0 false))))
    (:then_1
      (Utilities|FlowControl|DoOnce false) ; enters at Reset
    )))

(event EventDeactivate
  (params (NewCamera :type Actor%20Object%20Reference))
  (bind _returnvalue (Utilities|IsValid NewCamera))
  ;[1 1 1] Activating and deactivating the camera for setting the view target with blend and updating the isActive bool
  (Utilities|FlowControl|Sequence
    (:then_0
      (Utilities|FlowControl|DoOnce false
        (:Completed
          (Variables|Default|SetisActive false)
          (Game|Player|SetViewTargetwithBlend (Game|GetPlayerController 0) (select _returnvalue NewCamera (Game|GetPlayerCharacter 0)) 1.0 "VTBlend_Linear" 0.0 false)
          (CallFunction|UpdateinUse false (select _returnvalue NewCamera 0)))))
    (:then_1
      (Utilities|FlowControl|DoOnce false) ; enters at Reset
    )))

(fn ConstructionScript)